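; Main player controller that links the third-person character and the custom camera manager at startup.
; On BeginPlay it casts the controlled pawn to ThirdPersonCharacter and stores references in both directions.
; It then hands the Player_Camera_Manager to the character and calls that manager's OnPossess with controller and player.
; Camera-side failures print debug strings, while a failed pawn cast stops silently because its print is unwired.
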(event `self.ReceiveBeginPlay`
  (bind _returnvalue (`self.K2_GetPawn`))
  ;[1 1 1] Begin play
  ;;[1 1 1] Player
  (`/Engine/EditorBlueprintResources/StandardMacros.IsValid` _returnvalue
    (:`Is Valid`
      (bind _asthird_person_character (cast `/Game/Blueprint/ThirdPersonCharacter` _returnvalue))
      (bind _output_get (set `self.Player-Ref` _asthird_person_character))
      (set `/Game/Blueprint/ThirdPersonCharacter.Player controller` self _output_get)
      ;;[1 1 1] Camera Manager
      (bind _asplayer_camera_manager (cast `/Game/Blueprint/Base/Camera_System/Player_Camera_Manager` (`self.PlayerCameraManager`))
        (:`then`
          (bind _output_get_2 (set `self.Camera Manager` _asplayer_camera_manager))
          (bind _player_ref (`self.Player-Ref`)
            (:`then`
              (bind _output_get_3 (set `/Game/Blueprint/ThirdPersonCharacter.Camera Manager` _output_get_2 _player_ref))
              (`/Game/Blueprint/Base/Camera_System/Player_Camera_Manager.OnPossess` _output_get_3 self _player_ref))
            (:`else`
              (`KismetSystemLibrary.PrintString` "(Third person character) is not Valid From (Main Player Controller)"))))
        (:`CastFailed`
          (`KismetSystemLibrary.PrintString` "Faild to cast to (Player_Camera_Manager) From ( Main Player Controller)"))))))

(fn `UserConstructionScript`)