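; Spawner actor that keeps one weapon, item or bot present at its transform, chosen by ActorToSpawn.
; It spawns on BeginPlay, only on the server, passing class-default data to weapons and items.
; A looping timer respawns when the tracked actor becomes invalid.
; Dead bots are destroyed after a short delay, then replaced.
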(event `self.ReceiveBeginPlay`
  ;[1 1 1] BeginPlay
  (`self.Spawn`)
  (`KismetSystemLibrary.K2_SetTimerDelegate` (delegate `Update`) 3.0 true))

(event `Update`
  ;[1 1 1] Update
  (switch `/Game/Blueprint/Data/Enum/Actors` (`self.Actor to spawn`)
    (:`NewEnumerator0`
      (`self.Current Weapon`
        (:`then`)
        (:`else`
          (`self.Spawn` :!label _label))))
    (:`NewEnumerator1`
      (`self.Current Item`
        (:`then`)
        (:`else`
          (goto _label))))
    (:`NewEnumerator2`
      (bind _current_bot (`self.Current Bot`)
        (:`then`
          (if (`/Game/Blueprint/AI/AI_Character.Is Dead` _current_bot)
            (`KismetSystemLibrary.Delay` 3.0)
            (bind _current_bot_2 (`self.Current Bot`)
              (:`then`
                (`self.K2_DestroyActor` _current_bot_2)
                (goto _label))
              (:`else`))))
        (:`else`
          (goto _label))))))

(event `Spawn`
  (bind _returnvalue (`self.GetTransform`))
  (bind _weapon (`self.Weapon`))
  (bind _item (`self.Item`))
  (bind (_item_data _weapon_kind) (defaults `Object` _item))
  (bind (_weapon_data _single_shot) (defaults `Object` _weapon))
  ;[1 1 1] Spawn
  (if (`KismetSystemLibrary.IsServer`)
    (switch `/Game/Blueprint/Data/Enum/Actors` (`self.Actor to spawn`)
      (:`NewEnumerator0`
        (bind _returnvalue_2 (`|SpawnActorFromClass` _weapon _returnvalue "Undefined" "OverrideRootScale" null null null _weapon_data _single_shot (struct) "NewEnumerator3" null))
        (set `self.Current Weapon` _returnvalue_2))
      (:`NewEnumerator1`
        (bind _returnvalue_3 (`|SpawnActorFromClass` _item _returnvalue "Undefined" "OverrideRootScale" null _item_data null _weapon_kind null))
        (set `self.Current Item` _returnvalue_3))
      (:`NewEnumerator2`
        (bind _returnvalue_4 (`|SpawnActorFromClass` (`self.Bot`) _returnvalue "Undefined" "OverrideRootScale" null null null))
        (set `self.Current Bot` _returnvalue_4)))))

(fn `UserConstructionScript`)