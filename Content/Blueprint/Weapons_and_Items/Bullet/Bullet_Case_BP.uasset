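; Bullet case actor that spins briefly after spawning, then falls and removes itself.
; On begin play it applies its mesh and rotation, and a looping timer at frame delta adds random yaw to the skeletal mesh.
; After a short delay it stops projectile movement, enables gravity, physics simulation and a sound-spawn flag, and clears the spin timer.
; The actor destroys itself a few seconds later.
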(event `self.ReceiveBeginPlay`
  (bind _projectilemovement (`self.ProjectileMovement`))
  ;[1 1 1] begin Play
  (`SkinnedMeshComponent.SetSkinnedAssetAndUpdate` (`self.SkeletalMesh`) (`self.Mesh`) true)
  (`SceneComponent.K2_SetWorldRotation` (`self.SkeletalMesh`) (`self.Skeletal Mesh Rotation`) false false)
  (`KismetSystemLibrary.K2_SetTimerDelegate` (delegate `Rotate Bullet Case`) (`GameplayStatics.GetWorldDeltaSeconds`) true)
  (`KismetSystemLibrary.Delay` 0.3)
  (`|ExecutionSequence`
    (:`then_0`
      (`MovementComponent.StopMovementImmediately` _projectilemovement)
      (set `ProjectileMovementComponent.ProjectileGravityScale` 1.0 _projectilemovement)
      (set `self.can Spawn Sound` true))
    (:`then_1`
      (`PrimitiveComponent.SetSimulatePhysics` (`self.SkeletalMesh`) true))
    (:`then_2`
      (`KismetSystemLibrary.K2_SetTimerDelegate` (delegate `Rotate Bullet Case`))
      (`KismetSystemLibrary.Delay` 3.0)
      (`self.K2_DestroyActor`))))

(event `Rotate Bullet Case`
  ;[1 1 1] update
  (`SceneComponent.K2_SetWorldRotation` (`self.SkeletalMesh`) (`KismetMathLibrary.MakeRotator` (.roll (`SceneComponent.K2_GetComponentRotation` (`self.SkeletalMesh`))) (.pitch (`SceneComponent.K2_GetComponentRotation` (`self.SkeletalMesh`))) (+ (.yaw (`SceneComponent.K2_GetComponentRotation` (`self.SkeletalMesh`))) (`KismetMathLibrary.RandomFloatInRange` 30.0 50.0))) false true))

(fn `UserConstructionScript`)