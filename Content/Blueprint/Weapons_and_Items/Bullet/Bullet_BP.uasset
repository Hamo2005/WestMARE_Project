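; Projectile bullet actor that damages bodies through the TakeDamage interface and can penetrate surfaces, with Speed derived from its damage value.
; On bounce, a line trace identifies the physical material, spawning its mapped effect and sound plus a bullet-hole decal.
; For penetrable materials, a reverse sphere trace finds the exit point and spawns a replacement bullet there with damage recomputed by DegressDamage, then destroys itself.
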(event `self.ReceiveBeginPlay`
  ;[1 1 1] begin play
  (`SkinnedMeshComponent.SetSkinnedAssetAndUpdate` (`self.SkeletalMesh`) (`self.Mesh`) true)
  (`KismetSystemLibrary.K2_SetTimer` null "Set Damage By Time" 0.1 true)
  (set `self.Speed` (* (`self.Damage Value`) 100))
  (`self.SetLifeSpan` 60.0))

(event `self.ProjectileMovement.OnProjectileBounce`
  (params (ImpactResult :type "HitResult Structure (by ref)") (ImpactVelocity :type "Vector Structure (by ref)"))
  (bind _pawn (`self.Pawn`))
  ;[1 1 1] Impact
  (bind (_outhit _returnvalue) (`KismetSystemLibrary.LineTraceSingle` (`SceneComponent.K2_GetComponentLocation` (`self.Trace Start Location0`)) (`SceneComponent.K2_GetComponentLocation` (`self.Trace End Location`)) "TraceTypeQuery1" false (`|MakeArray` (`self.Pawn`) :!type "Actor Object Reference")))
  (if _returnvalue
    (`/Engine/EditorBlueprintResources/StandardMacros.DoOnce` false
      (:`Completed`
        (bind (_bblockinghit _binitialoverlap _time _distance _location _impactpoint _normal _impactnormal _physmat _hitactor _hitcomponent _hitbonename) (`GameplayStatics.BreakHitResult` _outhit))
        (`self.Effect,Sound and bullet Hole at Fire Location` _location _physmat _hitcomponent _impactnormal)
        (if (== _physmat "/Game/Content/PhysicalMaterials/M_BodyDamage.M_BodyDamage")
          (`self.Damage` _hitactor _hitbonename)
          (`self.K2_DestroyActor` :!label _label)
          (else
            (bind (_value _returnvalue_2) (`BlueprintMapLibrary.Map_Find` (`self.Phys Mat Damage`) _physmat))
            (if _returnvalue_2
              (if (== _value 0)
                (goto _label)
                (elif (>= (`self.Damage Value`) _value)
                  (if (<= (`self.Damage Value`) 1)
                    (goto _label)
                    (else
                      ;[1 1 1] Compute Exit Location
                      (bind _exit_location (`self.Compute Exit Location` ImpactResult))
                      (set `self.Damage Value` (`KismetMathLibrary.FTrunc` (- (`self.Damage Value`) (/ (`KismetMathLibrary.VSize` (- _exit_location (`.Location` (`GameplayStatics.BreakHitResult` ImpactResult)))) 10.0))))
                      (if (not (<= (`self.Damage Value`) 0))
                        (`|SpawnActorFromClass` "Bullet_BP_C" (`KismetMathLibrary.MakeTransform` _exit_location (`KismetMathLibrary.FindLookAtRotation` _exit_location (`self.Weapon Trace End`))) "Undefined" "OverrideRootScale" _pawn (`self.Damage Value`) _pawn (`self.Weapon Trace End`) (`self.Weapon Master`) (`self.Mesh`) null))
                      (`self.K2_DestroyActor`)))
                  (else
                    (goto _label))))
              (else
                (goto _label)))))))
    (else
      (goto _label))))

(event `self.Sound Sphere.OnComponentBeginOverlap`
  (params (OverlappedComponent :type "PrimitiveComponent Object Reference") (OtherActor :type "Actor Object Reference") (OtherComp :type "PrimitiveComponent Object Reference") (OtherBodyIndex :type Integer) (bFromSweep :type Boolean) (SweepResult :type "HitResult Structure (by ref)"))
  ;[1 1 1] play sound near othe players player
  (`GameplayStatics.PlaySoundAtLocation` null (`self.K2_GetActorLocation`) (struct) 1.0 1.0 0.0 null null null))

(fn `Compute Exit Location`
  (params (`Hit Result` :type "HitResult Structure"))
  (returns (`Exit Location` :type "Vector Structure") (`Result Found` :type Boolean))
  (bind (_bblockinghit _binitialoverlap _time _distance _location _impactpoint _normal _impactnormal _physmat _hitactor) (`GameplayStatics.BreakHitResult` `Hit Result`))
  ;[1 1 1] Compute Exit Location
  (bind _outhits (`KismetSystemLibrary.SphereTraceMultiForObjects` (`self.Weapon Trace End`) _location 0.0 (`|MakeArray` "ObjectTypeQuery1" "ObjectTypeQuery2" "ObjectTypeQuery3" "ObjectTypeQuery4" "ObjectTypeQuery5" "ObjectTypeQuery6" :!type "EObjectTypeQuery Enum")))
  (for _array_element _outhits
    (bind (_bblockinghit_2 _binitialoverlap_2 _time_2 _distance_2 _location_2 _impactpoint_2 _normal_2 _impactnormal_2 _physmat_2 _hitactor_2) (`GameplayStatics.BreakHitResult` _array_element))
    (if (== _hitactor_2 _hitactor)
      (return _location_2 true)))
  (return (0.0 0.0 0.0) false))

(fn `Damage`
  (params (`Hit Actor` :type "Object Object Reference") (`Bone Name` :type Name))
  (if (`KismetSystemLibrary.DoesImplementInterface` `Hit Actor` "/Game/Blueprint/Data/Interfaces/TakeDamage.TakeDamage_C")
    (message `/Game/Blueprint/Data/Interfaces/TakeDamage.ITakeDamage` `Hit Actor` `Bone Name` (`self.Damage Value`) (`self.Pawn`))
    (return)))

(fn `Effect,Sound and bullet Hole at Fire Location`
  (params (Location :type "Vector Structure") (Physical :type "PhysicalMaterial Object Reference") (`Hit Component` :type "PrimitiveComponent Object Reference") (`Impact Normal` :type "Vector Structure"))
  (bind (_value _returnvalue) (`BlueprintMapLibrary.Map_Find` (`self.Bullet Effect`) Physical))
  (bind (_value_2 _returnvalue_2) (`BlueprintMapLibrary.Map_Find` (`self.Bullet Sound`) Physical))
  ;[1 1 1] Effect and Sound at Fire Location and Bullet hole
  (`|ExecutionSequence`
    (:`then_0`
      (if _returnvalue
        (`/Engine/EditorBlueprintResources/StandardMacros.IsValid` _value
          (:`Is Valid`
            (`GameplayStatics.SpawnEmitterAtLocation` _value Location)))))
    (:`then_1`
      (if _returnvalue_2
        (`/Engine/EditorBlueprintResources/StandardMacros.IsValid` _value_2
          (:`Is Valid`
            (`GameplayStatics.PlaySoundAtLocation` _value_2 Location (struct) 1.0 1.0 0.0 "/Game/Content/Audio/Audio_Settings/Attenuation/Ambient_OneShot.Ambient_OneShot" "/Game/Content/Audio/Audio_Settings/Concurrency/SCon_Default.SCon_Default" null)))))
    (:`then_2`
      (if (`.ReturnValue` (`BlueprintMapLibrary.Map_Find` (`self.bullet Hole`) Physical))
        _
        (else
          _))
      (`GameplayStatics.SpawnDecalAttached` "/Game/Weapon-Items/Bullets/Bullet_Holes/Normal/M_Normal_BulletHole.M_Normal_BulletHole" (15.0 15.0 15.0) `Hit Component` "None" Location (`KismetMathLibrary.Conv_VectorToRotator` `Impact Normal`) "KeepWorldPosition" 3.0))))

(fn `Increse Damage By Time`
  (if (not (<= (`self.Damage Value`) 1))
    (set `self.Damage Value` (- (`self.Damage Value`) -1))))

(fn `OnRep_Damage Value`
  (set `self.Speed` (* (`self.Damage Value`) 100)))

(fn `UserConstructionScript`)