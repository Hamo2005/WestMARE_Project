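; Weapon magazine actor that shows a full or empty skeletal mesh depending on its current ammo.
; On BeginPlay, a SimulatePhysics flag either turns the Cube into a physics-only body that blocks WorldStatic or disables its collision and physics.
; The mesh is chosen at BeginPlay and again in the CurrentAmmo RepNotify, so the visual follows replicated ammo changes.
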(event `self.ReceiveBeginPlay`
  (bind _cube (`self.Cube`))
  ;[1 1 1] Collision
  (if (`self.simulate Physics`)
    (`PrimitiveComponent.SetCollisionEnabled` _cube "PhysicsOnly")
    (`PrimitiveComponent.SetSimulatePhysics` _cube true)
    (`PrimitiveComponent.SetCollisionResponseToChannel` _cube "ECC_WorldStatic" "ECR_Block")
    (else
      (`PrimitiveComponent.SetCollisionEnabled` _cube "NoCollision")
      (`PrimitiveComponent.SetSimulatePhysics` _cube false)
      (`PrimitiveComponent.SetCollisionResponseToChannel` _cube "ECC_WorldStatic" "ECR_Ignore")))
  (if (<= (`self.Current Ammo`) 0)
    (`SkinnedMeshComponent.SetSkinnedAssetAndUpdate` (`self.SkeletalMesh`) (`self.Empty Mag`) true)
    (else
      (`SkinnedMeshComponent.SetSkinnedAssetAndUpdate` (`self.SkeletalMesh`) (`self.Full Mag`) true))))

(fn `OnRep_Current Ammo`
  (if (<= (`self.Current Ammo`) 0)
    (`SkinnedMeshComponent.SetSkinnedAssetAndUpdate` (`self.SkeletalMesh`) (`self.Empty Mag`) true)
    (else
      (`SkinnedMeshComponent.SetSkinnedAssetAndUpdate` (`self.SkeletalMesh`) (`self.Full Mag`) true))))

(fn `UserConstructionScript`)