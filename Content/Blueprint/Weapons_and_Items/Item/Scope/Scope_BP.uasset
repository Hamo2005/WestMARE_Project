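; Scope item that drives its own aim-down-sights camera, setting its FOV and item name on BeginPlay.
; Each tick while the player is not firing, the camera eases toward the mesh's ADS socket with sway from player turn and look input.
; ADSFire uses the same follow with randomized recoil, stronger for Sniper, Shotgun and Pistol than for AR and SMG.
; Both paths rotate the camera toward the FinalADS point with roll locked.
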(event `self.ReceiveBeginPlay`
  ;[1 1 1] Event Begin play
  (`parent.ReceiveBeginPlay`)
  (`CameraComponent.SetFieldOfView` (`self.ADS Camera`) (`self.FOV`))
  (set `self.Name` (`.ItemName_39_BAA7C6844F9F76CFEB07339740F6053E` (break `/Game/Blueprint/Weapons_and_Items/Item/Data/Struc/Item_Data` (`self.Item Data`)))))

(event `self.ReceiveTick`
  (params (DeltaSeconds :type "Float (single-precision)"))
  (bind _returnvalue_location (`KismetMathLibrary.BreakTransform` (`SceneComponent.GetSocketTransform` (`self.SkeletalMesh`) "ADS" "RTS_Actor")))
  (bind _returnvalue_location_2 (`KismetMathLibrary.BreakTransform` (`SceneComponent.GetRelativeTransform` (`self.ADS Camera`))))
  (bind (__x__out __y__out __z__out) (`self.ADS Sway` (.x (`KismetMathLibrary.VInterpTo` _returnvalue_location_2 _returnvalue_location (`GameplayStatics.GetWorldDeltaSeconds`) 3.0)) (.y (`KismetMathLibrary.VInterpTo` _returnvalue_location_2 _returnvalue_location (`GameplayStatics.GetWorldDeltaSeconds`) 3.0)) (.z (`KismetMathLibrary.VInterpTo` _returnvalue_location_2 _returnvalue_location (`GameplayStatics.GetWorldDeltaSeconds`) 3.0))))
  ;[1 1 1] Update
  (`self.Player-Ref`
    (:`then`
      (if (not (`/Game/Blueprint/ThirdPersonCharacter.Fire` (`self.Player-Ref`)))
        (`SceneComponent.K2_SetRelativeLocationAndRotation` (`self.ADS Camera`) (`KismetMathLibrary.MakeVector` __x__out __y__out __z__out) (`KismetMathLibrary.MakeRotator` 0.0 (.pitch (`KismetMathLibrary.FindLookAtRotation` _returnvalue_location_2 (`SceneComponent.RelativeLocation` (`self.FinalADS`)))) (.yaw (`KismetMathLibrary.FindLookAtRotation` _returnvalue_location_2 (`SceneComponent.RelativeLocation` (`self.FinalADS`))))) true false)))
    (:`else`)))

(event `ADS Fire`
  (bind _returnvalue_location (`KismetMathLibrary.BreakTransform` (`SceneComponent.GetSocketTransform` (`self.SkeletalMesh`) "ADS" "RTS_Actor")))
  (bind _returnvalue_location_2 (`KismetMathLibrary.BreakTransform` (`SceneComponent.GetRelativeTransform` (`self.ADS Camera`))))
  (bind (__y__out __z__out __x__out) (`self.ADS Sway Fire` (.z (`KismetMathLibrary.VInterpTo` _returnvalue_location_2 _returnvalue_location (`GameplayStatics.GetWorldDeltaSeconds`) 3.0)) (.y (`KismetMathLibrary.VInterpTo` _returnvalue_location_2 _returnvalue_location (`GameplayStatics.GetWorldDeltaSeconds`) 3.0)) (.x (`KismetMathLibrary.VInterpTo` _returnvalue_location_2 _returnvalue_location (`GameplayStatics.GetWorldDeltaSeconds`) 3.0))))
  ;[1 1 1] Update
  (`SceneComponent.K2_SetRelativeLocationAndRotation` (`self.ADS Camera`) (`KismetMathLibrary.MakeVector` __x__out __y__out __z__out) (`KismetMathLibrary.MakeRotator` 0.0 (.pitch (`KismetMathLibrary.FindLookAtRotation` _returnvalue_location_2 (`SceneComponent.RelativeLocation` (`self.FinalADS`)))) (.yaw (`KismetMathLibrary.FindLookAtRotation` _returnvalue_location_2 (`SceneComponent.RelativeLocation` (`self.FinalADS`))))) true false))

(fn `ADS Sway`
  (params (`(X)` :type "Float (double-precision)") (`(Y)` :type "Float (double-precision)") (`(Z)` :type "Float (double-precision)"))
  (returns (`(X) out` :type "Float (double-precision)") (`(Y) out` :type "Float (double-precision)") (`(Z) out` :type "Float (double-precision)"))
  (bind _returnvalue (`GameplayStatics.GetWorldDeltaSeconds`))
  (bind _player_ref (`self.Player-Ref`))
  (bind __z_ (`local.(Z)`))
  (bind __y_ (`local.(Y)`))
  (return (`local.(X)`) (`KismetMathLibrary.FInterpTo` __y_ (- __y_ (* -1 (`/Game/Blueprint/ThirdPersonCharacter.Turn (Yaw)` _player_ref))) _returnvalue 1.0) (`KismetMathLibrary.FInterpTo` __z_ (- __z_ (`/Game/Blueprint/ThirdPersonCharacter.Look Up (Pitch)` _player_ref)) _returnvalue 1.0)))

(fn `ADS Sway Fire`
  (params (`(Z)` :type "Float (double-precision)") (`(Y)` :type "Float (double-precision)") (`(X)` :type "Float (double-precision)"))
  (returns (`(Y) out` :type "Float (double-precision)") (`(Z) out` :type "Float (double-precision)") (`(X) out` :type "Float (double-precision)"))
  (locals (`Pitch interp Speed` :type "Float (double-precision)" :default 0.0) (`Z Random in Range` :type "Float (double-precision)" :default 0.0) (`X Target` :type "Float (double-precision)") (`X interp Speed` :type "Float (double-precision)"))
  (bind _returnvalue (`GameplayStatics.GetWorldDeltaSeconds`))
  (bind __z_ (`local.(Z)`))
  (bind __y_ (`local.(Y)`))
  (bind __x_ (`local.(X)`))
  (bind _player_ref (`self.Player-Ref`)
    (:`then`
      (switch `/Game/Blueprint/Weapons_and_Items/Weapon/Data/Enum/Weapon_Kind` (`self.Weapon Kind`)
        (:`NewEnumerator5`
          (`KismetSystemLibrary.PrintString` "Weapon Kind is (None) From Scope_BP"))
        (:`NewEnumerator0`
          (set `local.Pitch interp Speed` 3.0 :!label _label)
          (set `local.Z Random in Range` (`KismetMathLibrary.RandomFloatInRange` (+ __z_ 0.5) (+ __z_ 1.0)))
          (set `local.X interp Speed` 10.0)
          (set `local.X Target` (`KismetMathLibrary.RandomFloatInRange` (+ __x_ 0.0) (+ __x_ 0.05)))
          (return (`KismetMathLibrary.FInterpTo` __y_ (- (`KismetMathLibrary.RandomFloatInRange` (- __y_ 2.0) (+ __y_ 2.0)) (* -1 (`/Game/Blueprint/ThirdPersonCharacter.Turn (Yaw)` _player_ref))) _returnvalue 1.0) (`KismetMathLibrary.FInterpTo` (`local.(Z)`) (- (`local.Z Random in Range`) (`/Game/Blueprint/ThirdPersonCharacter.Look Up (Pitch)` _player_ref)) _returnvalue (`local.Pitch interp Speed`)) (`KismetMathLibrary.FInterpTo` (`local.(X)`) (`local.X Target`) _returnvalue (`local.X interp Speed`))))
        (:`NewEnumerator1`
          (set `local.Pitch interp Speed` 10.0 :!label _label_2)
          (set `local.Z Random in Range` (`KismetMathLibrary.RandomFloatInRange` (+ __z_ 1.0) (+ __z_ 2.0)))
          (set `local.X interp Speed` 30.0)
          (set `local.X Target` (`KismetMathLibrary.RandomFloatInRange` (+ __x_ 0.0) (+ __x_ 0.5)))
          (return (`KismetMathLibrary.FInterpTo` __y_ (- (`KismetMathLibrary.RandomFloatInRange` (- __y_ 2.0) (+ __y_ 2.0)) (* -1 (`/Game/Blueprint/ThirdPersonCharacter.Turn (Yaw)` _player_ref))) _returnvalue 1.0) (`KismetMathLibrary.FInterpTo` (`local.(Z)`) (- (`local.Z Random in Range`) (`/Game/Blueprint/ThirdPersonCharacter.Look Up (Pitch)` _player_ref)) _returnvalue (`local.Pitch interp Speed`)) (`KismetMathLibrary.FInterpTo` (`local.(X)`) (`local.X Target`) _returnvalue (`local.X interp Speed`))))
        (:`NewEnumerator2`
          (goto _label_2))
        (:`NewEnumerator3`
          (goto _label_2))
        (:`NewEnumerator4`
          (goto _label))))
    (:`else`)))

(fn `UserConstructionScript`
  (`parent.UserConstructionScript`))