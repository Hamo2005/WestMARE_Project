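; AI controller for shooter bots that drives an AI_Character to find weapons and ammo, hunt enemies and fight.
; Each Tick copies the bot's state, writes back aim and needed ammo types, then runs a hand-built decision tree instead of a Behavior Tree.
; Branches use AI MoveTo toward enemies, pickups or random nav points, jumping when a move fails.
; Fire runs after enemy moves, shooting only when stationary with an enemy visible.
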(event `Fire`
  (bind _bot_ref (`self.Bot-Ref`))
  ;[1 1 1] Custom Event
  (if (`self.Is Moving`)
    (`/Game/Blueprint/AI/AI_Character.AI_WeaponFire_OFF` _bot_ref :!label _label)
    (elif (`self.See Enemy`)
      (`/Game/Blueprint/AI/AI_Character.AI_WeaponFire_ON` _bot_ref)
      (`|ExecutionSequence`
        (:`then_0`
          (bind _currentweapon (`/Game/Blueprint/AI/AI_Character.CurrentWeapon` _bot_ref)
            (:`then`
              (if (== (`.CurrentAmmo_11_A09B9A5A4840AEBF05B05A93225DF557` (break `/Game/Blueprint/Weapons_and_Items/Weapon/Data/Struc/Weapon_Data` (`/Game/Blueprint/Weapons_and_Items/Weapon/Weapon_Master.Weapon Data` _currentweapon))) 0)
                (`self.Search For Ammo When Firing`)))
            (:`else`)))
        (:`then_1`
          (if (`self.There Is A Bot/Player Near`)
            (`self.Keep Distance While Firing`))))
      (else
        (goto _label)))))

(event `self.ReceiveTick`
  (params (DeltaSeconds :type "Float (single-precision)"))
  (bind _bot_ref (`self.Bot-Ref`))
  (bind _weapons_in_map (`self.Weapons In Map`))
  (bind _bot_ref_2 (`self.Bot-Ref`))
  (bind _bot_ref_3 (`self.Bot-Ref`))
  (bind _bot_ref_4 (`self.Bot-Ref`))
  (bind _bot_ref_5 (`self.Bot-Ref`))
  (bind _bot_ref_6 (`self.Bot-Ref`))
  (bind _weapons_in_map_2 (`self.Weapons In Map`))
  (bind _items_in_map (`self.Items In Map`))
  (bind _bot_ref_7 (`self.Bot-Ref`))
  (bind _bot_ref_8 (`self.Bot-Ref`))
  ;[0 0.316 0.964] Update
  (bind _asai_character (cast `/Game/Blueprint/AI/AI_Character` (`self.K2_GetPawn`)))
  (bind _output_get (set `self.Bot-Ref` _asai_character))
  (`/Engine/EditorBlueprintResources/StandardMacros.IsValid` _output_get
    (:`Is Valid`
      (`|ExecutionSequence`
        (:`then_0`
          (`self.Get AI Data`)
          (`self.Get Needed Ammo Type`)
          (`self.Set Variables in Bot_BP`)
          (`self.Set Aim`)
          (`self.SetControlRotation` (`/Game/Blueprint/AI/AI_Character.ControlRotation` (`self.Bot-Ref`))))
        (:`then_1`
          ;[0 1 0] Weapons & Ammo
          (if (`/Game/Blueprint/AI/AI_Character.Is Dead` (`self.Bot-Ref`))
            _
            (elif (`self.Has Weapon`)
              (if (`self.Has Ammo For Weapon`)
                (`self.Equip Weapon That has Ammo`)
                ;[1 0 0] Enemy & Fire
                (if (`self.See Enemy`)
                  (if (`self.There Is A Bot/Player Near`) :!label _label
                    (if (not (`self.Is Moving`)) :!label _label_2
                      (`|AIMoveTo` (`self.Bot-Ref`) (`NavigationSystemV1.K2_GetRandomLocationInNavigableRadius` (`self.Bot-Loction`) 250.0 null "/Script/AIModule.NavFilter_AIControllerDefault") null 0.0 true
                        (:`OnFail`
                          (`|ExecutionSequence`
                            (:`then_0`
                              (`/Game/Blueprint/AI/AI_Character.AI_Jump Press` _bot_ref_8))
                            (:`then_1`
                              (`/Game/Blueprint/AI/AI_Character.AI_Jump Release` _bot_ref_8))))))
                    (elif (not (`self.Is Moving`))
                      (bind _enemy (`self.Enemy`)
                        (:`then`
                          (`|AIMoveTo` (`self.Bot-Ref`) (`self.K2_GetActorLocation` _enemy) _enemy (`KismetMathLibrary.RandomFloatInRange` 250.0 1000.0)
                            (:`OnSuccess`
                              _)
                            (:`OnFail`
                              (`|ExecutionSequence`
                                (:`then_0`
                                  (`/Game/Blueprint/AI/AI_Character.AI_Jump Press` _bot_ref))
                                (:`then_1`
                                  (`/Game/Blueprint/AI/AI_Character.AI_Jump Release` _bot_ref)))))
                          (`self.Fire`))
                        (:`else`))))
                  (elif (`self.Under Attac`)
                    (goto _label)
                    (elif (not (`self.Is Moving`))
                      (`|AIMoveTo` (`self.Bot-Ref`) (`NavigationSystemV1.K2_GetRandomLocationInNavigableRadius` (`self.Bot-Loction`) 1500.0 null "/Script/AIModule.NavFilter_AIControllerDefault") null 5.0 true
                        (:`OnFail`
                          (`|ExecutionSequence`
                            (:`then_0`
                              (`/Game/Blueprint/AI/AI_Character.AI_Jump Press` _bot_ref_4))
                            (:`then_1`
                              (`/Game/Blueprint/AI/AI_Character.AI_Jump Release` _bot_ref_4))))))))
                (else
                  (`|ExecutionSequence` :!label _label_3
                    (:`then_0`
                      (if (`self.Is Moving`)
                        _
                        (elif (`KismetArrayLibrary.Array_IsEmpty` _items_in_map)
                          (if (`KismetArrayLibrary.Array_IsEmpty` _weapons_in_map_2)
                            (if (not (`self.Is Moving`))
                              (`|AIMoveTo` (`self.Bot-Ref`) (`NavigationSystemV1.K2_GetRandomLocationInNavigableRadius` (`self.Bot-Loction`) 1500.0 null "/Script/AIModule.NavFilter_AIControllerDefault") null 3.0 true
                                (:`OnFail`
                                  (`|ExecutionSequence`
                                    (:`then_0`
                                      (`/Game/Blueprint/AI/AI_Character.AI_Jump Press` _bot_ref_6))
                                    (:`then_1`
                                      (`/Game/Blueprint/AI/AI_Character.AI_Jump Release` _bot_ref_6))))))
                            (else
                              (for _array_element _weapons_in_map_2
                                (`/Engine/EditorBlueprintResources/StandardMacros.IsValid` _array_element
                                  (:`Is Valid`
                                    (break))))
                              (if (not (`self.Is Moving`))
                                (`/Engine/EditorBlueprintResources/StandardMacros.IsValid` _array_element
                                  (:`Is Valid`
                                    (`|AIMoveTo` (`self.Bot-Ref`) (`self.K2_GetActorLocation` _array_element) _array_element 2.0 true
                                      (:`then`
                                        (if (`self.Can Pick UP Weapon Multi Trace`) :!label _label_4
                                          (`/Game/Blueprint/AI/AI_Character.AI_PickUp_Weapon` (`self.Bot-Ref`))
                                          (`self.Equip Weapon That has Ammo`)))
                                      (:`OnSuccess`
                                        (goto _label_4))
                                      (:`OnFail`
                                        (`|ExecutionSequence`
                                          (:`then_0`
                                            (`/Game/Blueprint/AI/AI_Character.AI_Jump Press` _bot_ref_5))
                                          (:`then_1`
                                            (`/Game/Blueprint/AI/AI_Character.AI_Jump Release` _bot_ref_5))))))))))
                          (else
                            (for _array_element_2 _items_in_map
                              (`/Engine/EditorBlueprintResources/StandardMacros.IsValid` _array_element_2
                                (:`Is Valid`
                                  (break))))
                            (if (not (`self.Is Moving`))
                              (`/Engine/EditorBlueprintResources/StandardMacros.IsValid` _array_element_2
                                (:`Is Valid`
                                  (`|AIMoveTo` (`self.Bot-Ref`) (`self.K2_GetActorLocation` _array_element_2) _array_element_2 2.0 true
                                    (:`then`
                                      (if (`self.Can Pick Up Item Multi Trace`) :!label _label_5
                                        (`/Game/Blueprint/AI/AI_Character.AI_pickUp_Item` (`self.Bot-Ref`) "NewEnumerator1" (`self.Needed Ammo Type Weapon 1`) (`self.Needed Ammo Type Weapon 2`) (`self.Needed Ammo Type Pistol`))))
                                    (:`OnSuccess`
                                      (goto _label_5))
                                    (:`OnFail`
                                      (`|ExecutionSequence`
                                        (:`then_0`
                                          (`/Game/Blueprint/AI/AI_Character.AI_Jump Press` _bot_ref_7))
                                        (:`then_1`
                                          (`/Game/Blueprint/AI/AI_Character.AI_Jump Release` _bot_ref_7))))))))))))
                    (:`then_1`
                      (if (`self.Can Pick Up Item Multi Trace`)
                        (`/Game/Blueprint/AI/AI_Character.AI_pickUp_Item` (`self.Bot-Ref`) "NewEnumerator1" (`self.Needed Ammo Type Weapon 1`) (`self.Needed Ammo Type Weapon 2`) (`self.Needed Ammo Type Pistol`)))))))
              (else
                (`|ExecutionSequence`
                  (:`then_0`
                    (if (`self.Is Moving`)
                      _
                      (elif (`KismetArrayLibrary.Array_IsEmpty` _weapons_in_map)
                        (if (not (`self.Is Moving`))
                          (`|AIMoveTo` (`self.Bot-Ref`) (`NavigationSystemV1.K2_GetRandomLocationInNavigableRadius` (`self.Bot-Loction`) 1500.0 null "/Script/AIModule.NavFilter_AIControllerDefault") null 3.0 true
                            (:`OnFail`
                              (`|ExecutionSequence`
                                (:`then_0`
                                  (`/Game/Blueprint/AI/AI_Character.AI_Jump Press` _bot_ref_2))
                                (:`then_1`
                                  (`/Game/Blueprint/AI/AI_Character.AI_Jump Release` _bot_ref_2))))))
                        (else
                          (`KismetSystemLibrary.Delay` 0.1)
                          (for _array_element_3 _weapons_in_map
                            (`/Engine/EditorBlueprintResources/StandardMacros.IsValid` _array_element_3
                              (:`Is Valid`
                                (break))))
                          (if (not (`self.Is Moving`))
                            (`/Engine/EditorBlueprintResources/StandardMacros.IsValid` _array_element_3
                              (:`Is Valid`
                                (`|AIMoveTo` (`self.Bot-Ref`) (`self.K2_GetActorLocation` _array_element_3) null 5.0 true
                                  (:`OnFail`
                                    (`|ExecutionSequence`
                                      (:`then_0`
                                        (`/Game/Blueprint/AI/AI_Character.AI_Jump Press` _bot_ref_3))
                                      (:`then_1`
                                        (`/Game/Blueprint/AI/AI_Character.AI_Jump Release` _bot_ref_3))))))))))))
                  (:`then_1`
                    (if (`self.Can Pick UP Weapon Multi Trace`)
                      (`/Game/Blueprint/AI/AI_Character.AI_PickUp_Weapon` (`self.Bot-Ref`)))))))))))))

(event `Keep Distance While Firing`
  ;[1 0 0] Enemy & Fire
  (goto _label_2))

(event `Search For Ammo When Firing`
  ;[0 1 0] Weapons & Ammo
  (goto _label_3))

(fn `Equip Weapon That has Ammo`
  (bind _bot_ref (`self.Bot-Ref`))
  ;[1 1 1] Equip Weapon that Has Ammo
  (if (`self.Weapon 1 Has Ammo`)
    (if (not (`self.Rifle 1 Equiped`))
      (`/Game/Blueprint/AI/AI_Character.AI_Equip/UnEquip_Weapon1` _bot_ref))
    (elif (`self.Weapon 2 Has Ammo`)
      (if (not (`self.Rifle 2 Equiped`))
        (`/Game/Blueprint/AI/AI_Character.AI_Equip/UnEquip_Weapon2` _bot_ref))
      (elif (`self.Pistol Has Ammo`)
        (if (not (`self.Pistol Equiped`))
          (`/Game/Blueprint/AI/AI_Character.AI_Equip/UnEquip_Pistol` _bot_ref))))))

(fn `Get AI Data`
  (bind _bot_ref (`self.Bot-Ref`))
  (bind _bot_ref_2 (`self.Bot-Ref`))
  (bind _bot_ref_3 (`self.Bot-Ref`))
  (bind _bot_ref_4 (`self.Bot-Ref`))
  (bind _bot_ref_5 (`self.Bot-Ref`))
  ;[1 1 1] Get AI Data
  (`|ExecutionSequence`
    (:`then_0`
      ;;[1 1 1] Bot Info
      (set `self.Bot-Loction` (`self.K2_GetActorLocation` _bot_ref_2))
      (set `self.Is Moving` (`/Game/Blueprint/AI/AI_Character.IsMoving` _bot_ref_2))
      (set `self.Is Sprinting` (`/Game/Blueprint/AI/AI_Character.Is Sprinting` _bot_ref_2)))
    (:`then_1`
      ;;[1 1 1] Weapon Info Bool Variables
      (set `self.Pistol Picked Up` (`/Game/Blueprint/AI/AI_Character.Pistol PickedUp` _bot_ref_5))
      (set `self.Rifle 1 Picked Up` (`/Game/Blueprint/AI/AI_Character.Rifle 1 PickedUp` _bot_ref_5))
      (set `self.Rifle 2 Picked Up` (`/Game/Blueprint/AI/AI_Character.Rifle 2 PickedUp` _bot_ref_5))
      (set `self.Pistol Equiped` (`/Game/Blueprint/AI/AI_Character.Pistol Equiped` _bot_ref_5))
      (set `self.Rifle 1 Equiped` (`/Game/Blueprint/AI/AI_Character.Rifle 1 Equiped` _bot_ref_5))
      (set `self.Rifle 2 Equiped` (`/Game/Blueprint/AI/AI_Character.Rifle 2 Equiped` _bot_ref_5)))
    (:`then_2`
      ;;[1 1 1] Weapon Info
      (set `self.Rifle 1` (`/Game/Blueprint/AI/AI_Character.Rifle 1` _bot_ref))
      (set `self.Rifle 2` (`/Game/Blueprint/AI/AI_Character.Rifle 2` _bot_ref))
      (set `self.Pistol` (`/Game/Blueprint/AI/AI_Character.Pistol` _bot_ref)))
    (:`then_3`
      ;;[1 1 1] Inventory and Pickup
      (set `self.Inventory` (`/Game/Blueprint/AI/AI_Character.Inventory` _bot_ref_4))
      (set `self.Can Pick UP Weapon Multi Trace` (`/Game/Blueprint/AI/AI_Character.Can PickUP Weapon MultiTrace` _bot_ref_4))
      (set `self.Can Pick Up Item Multi Trace` (`/Game/Blueprint/AI/AI_Character.Can PickUp Item Multi Trace` _bot_ref_4)))
    (:`then_4`
      ;;[1 1 1] AI
      (set `self.See Enemy` (`/Game/Blueprint/AI/AI_Character.See Enemy` _bot_ref_3))
      (set `self.There Is A Bot/Player Near` (`/Game/Blueprint/AI/AI_Character.There is a Bot/Player near` _bot_ref_3))
      (set `self.Enemy` (`/Game/Blueprint/AI/AI_Character.Enemy` _bot_ref_3))
      (set `self.Under Attac` (`/Game/Blueprint/AI/AI_Character.Under Attac` _bot_ref_3))
      (set `self.Weapons In Map` (`/Game/Blueprint/AI/AI_Character.Weapons In Map` _bot_ref_3))
      (set `self.Items In Map` (`/Game/Blueprint/AI/AI_Character.Items In Map` _bot_ref_3)))))

(fn `Get Needed Ammo Type`
  ;[1 1 1] Get Needed Ammo
  (if (or (`self.Pistol Picked Up`) (`self.Rifle 1 Picked Up`) (`self.Rifle 2 Picked Up`))
    (if (`self.Rifle 1 Equiped`)
      (set `self.Needed Ammo Type Weapon 1` (`.AmmoType_158_23DF14E344C4FDC26B2BD9B0DCE8957D` (break `/Game/Blueprint/Weapons_and_Items/Weapon/Data/Struc/Weapon_Data` (`/Game/Blueprint/Weapons_and_Items/Weapon/Weapon_Master.Weapon Data` (`self.Rifle 1`)))))
      (elif (`self.Rifle 2 Equiped`)
        (set `self.Needed Ammo Type Weapon 2` (`.AmmoType_158_23DF14E344C4FDC26B2BD9B0DCE8957D` (break `/Game/Blueprint/Weapons_and_Items/Weapon/Data/Struc/Weapon_Data` (`/Game/Blueprint/Weapons_and_Items/Weapon/Weapon_Master.Weapon Data` (`self.Rifle 2`)))))
        (elif (`self.Pistol Equiped`)
          (set `self.Needed Ammo Type Pistol` (`.AmmoType_158_23DF14E344C4FDC26B2BD9B0DCE8957D` (break `/Game/Blueprint/Weapons_and_Items/Weapon/Data/Struc/Weapon_Data` (`/Game/Blueprint/Weapons_and_Items/Weapon/Weapon_Master.Weapon Data` (`self.Pistol`)))))
          (elif (`self.Rifle 1 Picked Up`)
            (set `self.Needed Ammo Type Weapon 1` (`.AmmoType_158_23DF14E344C4FDC26B2BD9B0DCE8957D` (break `/Game/Blueprint/Weapons_and_Items/Weapon/Data/Struc/Weapon_Data` (`/Game/Blueprint/Weapons_and_Items/Weapon/Weapon_Master.Weapon Data` (`self.Rifle 1`)))))
            (elif (`self.Rifle 2 Picked Up`)
              (set `self.Needed Ammo Type Weapon 2` (`.AmmoType_158_23DF14E344C4FDC26B2BD9B0DCE8957D` (break `/Game/Blueprint/Weapons_and_Items/Weapon/Data/Struc/Weapon_Data` (`/Game/Blueprint/Weapons_and_Items/Weapon/Weapon_Master.Weapon Data` (`self.Rifle 2`)))))
              (elif (`self.Pistol Picked Up`)
                (set `self.Needed Ammo Type Pistol` (`.AmmoType_158_23DF14E344C4FDC26B2BD9B0DCE8957D` (break `/Game/Blueprint/Weapons_and_Items/Weapon/Data/Struc/Weapon_Data` (`/Game/Blueprint/Weapons_and_Items/Weapon/Weapon_Master.Weapon Data` (`self.Pistol`)))))))))))))

(fn `Has Ammo For Weapon`
  (returns (`Has Ammo for Weapon` :type Boolean))
  ;[1 1 1] Check If Bot Has Ammo For Every Weapon
  (if (or (`self.Rifle 1 Picked Up`) (`self.Rifle 2 Picked Up`) (`self.Pistol Picked Up`))
    (`|ExecutionSequence`
      (:`then_0`
        (if (`self.Rifle 1 Picked Up`)
          (bind _has_ammo (`self.Has Ammo?` (`self.Rifle 1`)))
          (set `self.Weapon 1 Has Ammo` _has_ammo)
          (else
            (set `self.Weapon 1 Has Ammo` false))))
      (:`then_1`
        (if (`self.Rifle 2 Picked Up`)
          (bind _has_ammo_2 (`self.Has Ammo?` (`self.Rifle 2`)))
          (set `self.Weapon 2 Has Ammo` _has_ammo_2)
          (else
            (set `self.Weapon 2 Has Ammo` false))))
      (:`then_2`
        (if (`self.Pistol Picked Up`)
          (bind _has_ammo_3 (`self.Has Ammo?` (`self.Pistol`)))
          (set `self.Pistol Has Ammo` _has_ammo_3)
          (else
            (set `self.Pistol Has Ammo` false))))
      (:`then_3`
        (if (or (`self.Weapon 1 Has Ammo`) (`self.Weapon 2 Has Ammo`) (`self.Pistol Has Ammo`))
          (return true)
          (else
            (return false)))))))

(fn `Has Ammo?`
  (params (Weapon :type "/Game/Blueprint/Weapons_and_Items/Weapon/Weapon_Master Object Reference"))
  (returns (`Has Ammo` :type Boolean))
  (bind _weapon_data (`/Game/Blueprint/Weapons_and_Items/Weapon/Weapon_Master.Weapon Data` Weapon))
  (`/Engine/EditorBlueprintResources/StandardMacros.IsValid` Weapon
    (:`Is Valid`
      (if (== (`.CurrentAmmo_11_A09B9A5A4840AEBF05B05A93225DF557` (break `/Game/Blueprint/Weapons_and_Items/Weapon/Data/Struc/Weapon_Data` _weapon_data)) 0)
        (for _array_element (`self.Inventory`)
          (if (`|EnumEquality` (`.AmmoType_158_23DF14E344C4FDC26B2BD9B0DCE8957D` (break `/Game/Blueprint/Weapons_and_Items/Weapon/Data/Struc/Weapon_Data` _weapon_data)) (`.AmmoType_36_816B09194F02AC984A0532B1F49141A7` (break `/Game/Blueprint/Weapons_and_Items/Item/Data/Struc/Item_Data` _array_element)))
            (return true)))
        (return false)
        (else
          (return true))))
    (:`Is Not Valid`
      (return true))))

(fn `Has Weapon`
  (returns (`Has Weapon` :type Boolean))
  ;[1 1 1] Check if Bot Has Any Weapons
  (if (or (`self.Rifle 1 Picked Up`) (`self.Rifle 2 Picked Up`) (`self.Pistol Picked Up`))
    (return true)
    (else
      (return false))))

(fn `Set Aim`
  (bind _bot_ref (`self.Bot-Ref`))
  ;[1 1 1] Set is Aimming or not
  (if (`self.See Enemy`)
    (if (`self.Is Moving`)
      (if (`self.Is Sprinting`)
        (set `/Game/Blueprint/AI/AI_Character.Aim` false _bot_ref)
        (else
          (set `/Game/Blueprint/AI/AI_Character.Aim` true _bot_ref :!label _label)))
      (else
        (goto _label)))
    (else
      (set `/Game/Blueprint/AI/AI_Character.Aim` false (`self.Bot-Ref`)))))

(fn `Set Variables in Bot_BP`
  (bind _bot_ref (`self.Bot-Ref`))
  ;[1 1 1] Set Variables in Bot_BP
  (set `/Game/Blueprint/AI/AI_Character.Needed Ammo Type Weapon 1` (`self.Needed Ammo Type Weapon 1`) _bot_ref)
  (set `/Game/Blueprint/AI/AI_Character.Needed Ammo Type Weapon 2` (`self.Needed Ammo Type Weapon 2`) _bot_ref)
  (set `/Game/Blueprint/AI/AI_Character.Needed Ammo Type pistol` (`self.Needed Ammo Type Pistol`) _bot_ref))

(fn `UserConstructionScript`)